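; Dual-wield dagger weapon actor for Conan Exiles that adds an off-hand dagger and glow effects to both blades.
; On BeginPlay it async-loads the item's static mesh into FakeDagger and attaches it to the character's secondary socket.
; TrailStart skips dedicated servers, creates a dynamic material for the chosen hand and plays its fade timeline, scaled to trail duration plus delay.
; The off-hand timeline handled here drives the weapon_glow parameter from GlowColor.
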(event `self.ReceiveBeginPlay`
  (`parent.ReceiveBeginPlay`)
  (`|ExecutionSequence`
    (:`then_0`
      (bind _object (`|LoadAsset` (`GameItem.VisualStaticMesh` (`self.OwnerItem`))))
      (`StaticMeshComponent.SetStaticMesh` (`self.FakeDagger`) _object)
      (bind _asconan_character (cast `ConanCharacter` (`self.GetOwner`)))
      (`SceneComponent.K2_AttachToComponent` (`self.FakeDagger`) (`Character.Mesh` _asconan_character) "Socket_Secondary" "KeepRelative" "KeepRelative" "KeepRelative" true))
    (:`then_1`
      (bind (_direction _fade) (`Timeline|dual_wield_weapon_glow_fade` :!via `Stop`)
        (:`Update`
          (`MaterialInstanceDynamic.SetVectorParameterValue` (`self.dualwield_dynamic_weapon_material`) "weapon_glow" (* (`self.glow_color`) _fade)))))))

(fn `TrailStart`
  (params (TrailColor :type "LinearColor Structure") (GlowColor :type "LinearColor Structure") (WeaponTrailIndex :type Integer) (Trailduration :type "Float (double-precision)") (Offhand :type Boolean) (Loop :type Boolean))
  (returns (Success :type Boolean))
  (locals (isOffhand :type Boolean :default false) (timeline_to_use :type "TimelineComponent Object Reference") (trailcol :type "LinearColor Structure") (traildur :type "Float (double-precision)") (Trail_to_use :type "ParticleSystemComponent Object Reference"))
  (bind _returnvalue (select `bool` (`local.isOffhand`) :`false` (`self.StaticWeaponMesh`) :`true` (`self.FakeDagger`)))
  (if (`KismetSystemLibrary.IsDedicatedServer`)
    (return false)
    (else
      (set `self.glow_color` GlowColor)
      (set `local.traildur` Trailduration)
      (set `local.isOffhand` Offhand)
      (bind _returnvalue_2 (`PrimitiveComponent.CreateDynamicMaterialInstance` _returnvalue 0 (`PrimitiveComponent.GetMaterial` _returnvalue 0)))
      (if (`local.isOffhand`)
        (set `self.dualwield_dynamic_weapon_material` _returnvalue_2)
        (else
          (set `self.dynamic_weapon_material` _returnvalue_2)))
      (bind _output_get (set `local.timeline_to_use` (select `bool` (`local.isOffhand`) :`false` (`self.weapon_glow_fade`) :`true` (`self.dual_wield_weapon_glow_fade`))))
      (`TimelineComponent.SetPlayRate` _output_get (/ 1.0 (+ (`local.traildur`) (`self.glow_fade_delay`))))
      (`TimelineComponent.PlayFromStart` _output_get)
      (return true))))

(fn `UserConstructionScript`
  (`parent.UserConstructionScript`))